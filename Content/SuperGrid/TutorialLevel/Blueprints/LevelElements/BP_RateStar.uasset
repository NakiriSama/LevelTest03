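; BP_RateStar is a tutorial level star actor whose static mesh can temporarily stop blocking the WorldStatic channel.
; The Star_Collsion event sets that response to Ignore, then restores Block after a delay unless the player is inside the Box.
; Box overlap events track the ThirdPersonCharacter in an Overlap flag, and exiting restores Block immediately, even if the delay is still running.
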(event OnComponentBeginOverlap(Box)
  (params (OverlappedComponent :type Primitive%20Component%20Object%20Reference) (OtherActor :type Actor%20Object%20Reference) (OtherComp :type Primitive%20Component%20Object%20Reference) (OtherBodyIndex :type Integer) (bFromSweep :type Boolean) (SweepResult :type Hit%20Result%20Structure%20%28by%20ref%29))
  (if (== OtherActor (.AsThird%20Person%20Character (Utilities|Casting|CastToThirdPersonCharacter (Game|GetPlayerCharacter 0))))
    (Variables|Default|SetOverlap? true)))

(event OnComponentEndOverlap(Box)
  (params (OverlappedComponent :type Primitive%20Component%20Object%20Reference) (OtherActor :type Actor%20Object%20Reference) (OtherComp :type Primitive%20Component%20Object%20Reference) (OtherBodyIndex :type Integer))
  (if (== OtherActor (.AsThird%20Person%20Character (Utilities|Casting|CastToThirdPersonCharacter (Game|GetPlayerCharacter 0))))
    (Variables|Default|SetOverlap? false)
    (Collision|SetCollisionResponsetoChannel (Variables|Default|GetStaticMesh) "ECC_WorldStatic" "ECR_Block")))

(event Custom|Star_Collsion
  (Collision|SetCollisionResponsetoChannel (Variables|Default|GetStaticMesh) "ECC_WorldStatic" "ECR_Ignore")
  (Utilities|FlowControl|Delay 5.0)
  (if (not (Variables|Default|GetOverlap?))
    (Collision|SetCollisionResponsetoChannel (Variables|Default|GetStaticMesh) "ECC_WorldStatic" "ECR_Block")))

(event EventBeginPlay)

(event EventActorBeginOverlap
  (params (OtherActor :type Actor%20Object%20Reference)))

(event EventTick
  (params (DeltaSeconds :type Float%20%28single-precision%29)))

(fn ConstructionScript)